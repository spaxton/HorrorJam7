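; BP_Narrator is a narrator character actor that holds a pose animation and can fade in and out.
; On BeginPlay it loops the assigned pose animation on its skeletal mesh at a configurable play rate, if one is set.
; Fadein plays a timeline and FadeOut reverses it, with each update driving the Opacity scalar parameter on the mesh materials through SetMeshOpacity.
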(event Custom|SetMeshOpacity
  (params (Opacity :type Float%20%28single-precision%29))
  (Rendering|Material|SetScalarParameterValueonMaterials (Variables|Default|GetSkeletalMesh) "Opacity" Opacity))

(event EventBeginPlay
  (bind _skeletalmesh (Variables|Default|GetSkeletalMesh))
  (bind _narratorposeanim (Variables|Default|GetNarratorPoseAnim)
    (:then
      (Components|Animation|PlayAnimation _skeletalmesh _narratorposeanim true)
      (Components|Timeline|SetPlayRate _skeletalmesh (Variables|Default|GetPoseAnimPlayRate)))
    (:else)))

(event EventFadeOut
  (bind _fadealpha (Timeline|Timeline_FadeChar Reverse)
    (:Update
      (CallFunction|SetMeshOpacity _fadealpha))))

(event EventFadein
  (bind _fadealpha (Timeline|Timeline_FadeChar Play)
    (:Update
      (CallFunction|SetMeshOpacity _fadealpha))))

(fn ConstructionScript)