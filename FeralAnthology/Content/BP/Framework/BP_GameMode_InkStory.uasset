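; Game mode for an Ink-driven campfire storytelling game, running the main menu, credits, story gallery and reading screens.
; Gallery selection pulls story data from a table and blends between per-story cameras while toggling narrator visibility.
; Reading feeds Ink text and choices to the UI, parsing embedded ">>>" commands for images, sounds, campfire colour and a trust display.
; It also crossfades music and observes the Ink "trust" variable.
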(event Custom|ShowGallerySelection
  (params (StoryIndex :type Integer) (BlendTime :type Float%20%28single-precision%29))
  (if (Utilities|Array|IsValidIndex (Variables|Story|GetInLevelStoryActors) StoryIndex)
    (bind _output_get (Variables|Story|SetCurrentStoryIndex StoryIndex))
    (bind _output_get_2 (Variables|Story|SetCurrentStoryActors (Utilities|Array|Get(acopy) (Variables|Story|GetInLevelStoryActors) _output_get)))
    (bind _output_get_3 (Variables|Story|SetCurrentStoryRowname (Utilities|Struct|BreakS_InLevelStoryActors _output_get_2)))
    (bind _returnvalue (Utilities|GetDataTableRow "/Game/Data/Data_Stories.Data_Stories" _output_get_3)
      (:then
        (Variables|Story|SetCurrentStoryData _returnvalue)
        (Game|Player|SetViewTargetwithBlend (Game|GetPlayerController 0) (Utilities|Struct|BreakS_InLevelStoryActors (Variables|Story|GetCurrentStoryActors)) BlendTime "VTBlend_EaseInOut" 1.0 false)
        (Utilities|FlowControl|RetriggerableDelay (- BlendTime 0.1))
        (bind _ui_storygallery (Variables|UI|GetUI_StoryGallery)
          (:then
            (Default|UpdateSelectionInfo _ui_storygallery (.Title (Utilities|Struct|BreakS_Story (Variables|Story|GetCurrentStoryData))) (.Author (Utilities|Struct|BreakS_Story (Variables|Story|GetCurrentStoryData))) (.Synopsis (Utilities|Struct|BreakS_Story (Variables|Story|GetCurrentStoryData))) (.Warnings (Utilities|Struct|BreakS_Story (Variables|Story|GetCurrentStoryData))) (.MinutesLength (Utilities|Struct|BreakS_Story (Variables|Story|GetCurrentStoryData))) (Variables|Story|GetCurrentStoryIndex) (Variables|Story|GetLastStoryIndex))
            (Variables|UI|SetCurrentUI (Variables|UI|GetUI_StoryGallery)))
          (:else)))
      (:RowNotFound
        (Development|PrintString (Utilities|String|Append "Error: Cannot find story data for " (Utilities|String|ToString(Name) (Variables|Story|GetCurrentStoryRowname))) true true "(R=1.000000,G=0.000000,B=0.000000,A=1.000000)" 1e+01)))
    (else
      (Development|PrintString (Utilities|String|Append "Error: Cannot find story actors for index " (Utilities|String|ToString(Integer) StoryIndex)) true true "(R=1.000000,G=0.000000,B=0.000000,A=1.000000)" 1e+01))))

(event Custom|ShowAllNarrators
  ;[1 1 1] Narrator Characters
  (for _array_element (Variables|Story|GetInLevelStoryActors)
    (Rendering|SetVisibility (Variables|/Script/Engine.SkeletalMeshActor|GetSkeletalMeshComponent (Utilities|Struct|BreakS_InLevelStoryActors _array_element)) true true)))

(event Custom|GoToCredits
  (bind _ui_credits (Variables|UI|GetUI_Credits))
  (Utilities|FlowControl|Delay 0.25)
  (bind _ui_credits_2 (Variables|UI|GetUI_Credits)
    (:then
      (Input|SetInputModeGameandUI (Game|GetPlayerController 0) _ui_credits_2 "DoNotLock" true)
      (Class|IUI|UI-Show(Message) _ui_credits)
      (Variables|UI|SetCurrentUI _ui_credits))
    (:else)))

(event Custom|GoToExitGame
  (CameraFades|StartCameraFade :self (Variables|/Script/Engine.PlayerController|GetPlayerCameraManager (Game|GetPlayerController 0)) :ToAlpha 1.0 :Duration 1.0 :bHoldWhenFinished true)
  (bind _currentui (Variables|UI|GetCurrentUI)
    (:then
      (Class|IUI|UI-Hide(Message) _currentui))
    (:else
      _))
  (Utilities|FlowControl|Delay 1.0)
  (Game|QuitGame 0 "Quit" false))

(event Custom|BackToMainMenu
  (Game|Player|SetViewTargetwithBlend (Game|GetPlayerController 0) (Variables|Camera|GetMainCamera) 1.0 "VTBlend_EaseInOut" 1.0 false)
  (Utilities|FlowControl|Delay 0.75)
  (bind _ui_mainmenu (Variables|UI|GetUI_MainMenu)
    (:then
      (Class|IUI|UI-Show(Message) _ui_mainmenu)
      (Variables|UI|SetCurrentUI _ui_mainmenu))
    (:else)))

(event Custom|BackFromCredits
  (bind _ui_mainmenu (Variables|UI|GetUI_MainMenu)
    (:then
      (Class|IUI|UI-Show(Message) _ui_mainmenu)
      (Variables|UI|SetCurrentUI _ui_mainmenu))
    (:else)))

(event Custom|BackFromReadStory
  (bind _ui_storygallery (Variables|UI|GetUI_StoryGallery)
    (:then
      (Input|SetInputModeGameandUI (Game|GetPlayerController 0) _ui_storygallery "DoNotLock" true)
      (CallFunction|ShowGallerySelection (Variables|Story|GetCurrentStoryIndex) 0.67)
      (Variables|Story|SetCurrentStory 0)
      (Variables|Story|SetCurrentStoryData "")
      (CallFunction|ShowOtherNarrators)
      (CallFunction|ClearVariableTracking)
      (CallFunction|ChangeMusictoMain)
      (CallFunction|ResetCampfire)
      (CallFunction|ShowGallerySelection (Variables|Story|GetCurrentStoryIndex) 0.67))
    (:else)))

(event Custom|HideAllNarrators
  ;[1 1 1] Narrator Characters
  (for _array_element (Variables|Story|GetInLevelStoryActors)
    (Rendering|SetVisibility (Variables|/Script/Engine.SkeletalMeshActor|GetSkeletalMeshComponent (Utilities|Struct|BreakS_InLevelStoryActors _array_element)) false true)))

(event Custom|ShowOtherNarrators
  ;[1 1 1] Narrator Characters
  (for (_array_element _array_index) (Variables|Story|GetInLevelStoryActors)
    (if (!= _array_index (Variables|Story|GetCurrentStoryIndex))
      (Rendering|SetVisibility (Variables|/Script/Engine.SkeletalMeshActor|GetSkeletalMeshComponent (Utilities|Struct|BreakS_InLevelStoryActors _array_element)) true true))))

(event Custom|HideOtherNarrators
  ;[1 1 1] Narrator Characters
  (for (_array_element _array_index) (Variables|Story|GetInLevelStoryActors)
    (if (!= _array_index (Variables|Story|GetCurrentStoryIndex))
      (Rendering|SetVisibility (Variables|/Script/Engine.SkeletalMeshActor|GetSkeletalMeshComponent (Utilities|Struct|BreakS_InLevelStoryActors _array_element)) false true))))

(event Custom|PrevStory
  (CallFunction|ShowGallerySelection (- (Math|Integer|SelectInt (Variables|Story|GetCurrentStoryIndex) (Variables|Story|GetLastStoryIndex) (> (Variables|Story|GetCurrentStoryIndex) 0)) 1) 0.67))

(event Custom|NextStory
  (CallFunction|ShowGallerySelection (Math|Integer|SelectInt (+ (Variables|Story|GetCurrentStoryIndex) 1) 0 (< (Variables|Story|GetCurrentStoryIndex) (Variables|Story|GetLastStoryIndex))) 0.67))

(event Custom|GoToStories
  (Variables|Story|SetCurrentStory 0)
  (Variables|Story|SetCurrentStoryData "")
  (bind _ui_storygallery (Variables|UI|GetUI_StoryGallery)
    (:then
      (Input|SetInputModeGameandUI (Game|GetPlayerController 0) _ui_storygallery "DoNotLock" true)
      (CallFunction|ShowGallerySelection (Variables|Story|GetCurrentStoryIndex) 1.0))
    (:else)))

(event EventBeginPlay
  (bind _returnvalue (UserInterface|CreateWidget "/Game/BP/UI/Menu/UI_MainMenu.UI_MainMenu_C" (Game|GetPlayerController 0)))
  (bind _output_get (Variables|UI|SetUI_MainMenu _returnvalue))
  (UserInterface|Viewport|AddtoViewport _output_get 0)
  (EventDispatchers|BindEventtoOnStoriesSelected (Variables|UI|GetUI_MainMenu) (EventDispatchers|CreateEvent :!event Custom|GoToStories))
  (EventDispatchers|BindEventtoOnCreditsSelected (Variables|UI|GetUI_MainMenu) (EventDispatchers|CreateEvent :!event Custom|GoToCredits))
  (EventDispatchers|BindEventtoOnExitSelected (Variables|UI|GetUI_MainMenu) (EventDispatchers|CreateEvent :!event Custom|GoToExitGame))
  (Input|SetInputModeGameandUI (Game|GetPlayerController 0) (Variables|UI|GetUI_MainMenu) "DoNotLock" true)
  (bind _returnvalue_2 (UserInterface|CreateWidget "/Game/BP/UI/Menu/UI_Credits.UI_Credits_C" (Game|GetPlayerController 0)))
  (bind _output_get_2 (Variables|UI|SetUI_Credits _returnvalue_2))
  (UserInterface|Viewport|AddtoViewport _output_get_2 1)
  (EventDispatchers|BindEventtoClose (Variables|UI|GetUI_Credits) (EventDispatchers|CreateEvent :!event Custom|BackFromCredits))
  (bind _returnvalue_3 (UserInterface|CreateWidget "/Game/BP/UI/Story/UI_StoryGallery.UI_StoryGallery_C" (Game|GetPlayerController 0)))
  (bind _output_get_3 (Variables|UI|SetUI_StoryGallery _returnvalue_3))
  (UserInterface|Viewport|AddtoViewport _output_get_3 2)
  (EventDispatchers|BindEventtoOnBacktoMain (Variables|UI|GetUI_StoryGallery) (EventDispatchers|CreateEvent :!event Custom|BackToMainMenu))
  (EventDispatchers|BindEventtoOnNext (Variables|UI|GetUI_StoryGallery) (EventDispatchers|CreateEvent :!event Custom|NextStory))
  (EventDispatchers|BindEventtoOnPrev (Variables|UI|GetUI_StoryGallery) (EventDispatchers|CreateEvent :!event Custom|PrevStory))
  (EventDispatchers|BindEventtoOnReadStory (Variables|UI|GetUI_StoryGallery) (EventDispatchers|CreateEvent :!event Custom|ReadStory))
  (bind _returnvalue_4 (UserInterface|CreateWidget "/Game/BP/UI/Story/UI_ReadStory.UI_ReadStory_C" (Game|GetPlayerController 0)))
  (bind _output_get_4 (Variables|UI|SetUI_ReadStory _returnvalue_4))
  (UserInterface|Viewport|AddtoViewport _output_get_4 3)
  (EventDispatchers|BindEventtoOnBacktoStoryGallery (Variables|UI|GetUI_ReadStory) (EventDispatchers|CreateEvent :!event Custom|BackFromReadStory))
  (EventDispatchers|BindEventtoOnChoiceSelected (Variables|UI|GetUI_ReadStory) (EventDispatchers|CreateEvent :!event Custom|SelectChoice)))

(event EventGM-Quit
  (CallFunction|GotoExitGame))

(event EventGM-Start
  (Utilities|FlowControl|Sequence
    (:then_0
      (bind _ui_mainmenu (Variables|UI|GetUI_MainMenu)
        (:then
          (Class|IUI|UI-Show(Message) _ui_mainmenu)
          (Variables|UI|SetCurrentUI _ui_mainmenu))
        (:else
          (Development|PrintString "Error: Main Menu not valid" true true "(R=1.000000,G=0.000000,B=0.000000,A=1.000000)" 1e+01))))
    (:then_1
      (bind _mainmusicloop (Variables|Audio|GetMainMusicLoop)
        (:then
          (bind _returnvalue (Audio|SpawnSound2D _mainmusicloop 1.0 1.0 0.0 0 false false))
          (bind _output_get (Variables|Default|SetMainMusicEmitter _returnvalue))
          (Audio|Parameter|SetFloatParameter _output_get "MusicMixAlpha" 0.0 :!class /Script/Engine.AudioComponent))
        (:else
          (Development|PrintString "Error: background music not valid" true true "(R=1.000000,G=0.000000,B=0.000000,A=1.000000)" 1e+01))))
    (:then_2
      (bind _campfireloop (Variables|Audio|GetCampfireLoop)
        (:then
          (bind _returnvalue_2 (Audio|SpawnSound2D _campfireloop 1.0 1.0 0.0 0 false false))
          (Variables|Default|SetCampfireAudioEmitter _returnvalue_2))
        (:else
          (Development|PrintString "Error: Campfire audio not valid" true true "(R=1.000000,G=0.000000,B=0.000000,A=1.000000)" 1e+01))))))

(event EventGM-SetMainCamera
  (params (MainCamera :type Camera%20Actor%20Object%20Reference))
  (Variables|Camera|SetMainCamera MainCamera))

(event EventGM-SetCampfireEmitter
  (params (CampfireEmitter :type Particle%20System%20Component%20Object%20Reference))
  (Variables|Default|SetCampfireEmitter CampfireEmitter)
  (CallFunction|ChangeCampfire "Default"))

(event EventGM-SetinLevelStoryActors
  (params (InLevelStoryActors :type Array%20of%20S%20in%20Level%20Story%20Actors%20Structures))
  (bind _output_get (Variables|Story|SetInLevelStoryActors InLevelStoryActors))
  (Variables|Story|SetLastStoryIndex (Utilities|Array|LastIndex _output_get)))

(event EventGM-SetShotCameras
  (params (ShotCameras :type Map%20of%20Names%20to%20Objects))
  (Variables|Camera|SetStoryShotCameras ShotCameras))

(event EventGM-CampfireColor
  (params (Color :type String))
  (CallFunction|ChangeCampfire Color))

(event Custom|ReadStory
  (bind _inlevelstoryactors (Variables|Story|GetInLevelStoryActors))
  (bind _currentstorydata (Variables|Story|GetCurrentStoryData))
  (bind _currentstoryindex (Variables|Story|GetCurrentStoryIndex))
  (bind (_title _author) (Utilities|Struct|BreakS_Story _currentstorydata))
  (bind _output (Utilities|Array|Get(acopy) _inlevelstoryactors _currentstoryindex))
  (bind _tellstorycamera (Utilities|Struct|BreakS_InLevelStoryActors _output))
  (Variables|Story|GetCurrentStory
    (:then)
    (:else
      (if (Utilities|IsValid _tellstorycamera)
        (CallFunction|HideOtherNarrators)
        (Game|Player|SetViewTargetwithBlend (Game|GetPlayerController 0) _tellstorycamera 0.67 "VTBlend_EaseInOut" 1.0 false)
        (CallFunction|ChangeMusictoStory)
        (Utilities|FlowControl|RetriggerableDelay 0.5)
        (bind _returnvalue (Class|Story|NewStory (Utilities|Struct|BreakS_Story (Variables|Story|GetCurrentStoryData))))
        (Variables|Story|SetCurrentStory _returnvalue)
        (Utilities|FlowControl|Sequence
          (:then_0
            (bind _ui_readstory (Variables|UI|GetUI_ReadStory)
              (:then
                (Input|SetInputModeGameandUI (Game|GetPlayerController 0) _ui_readstory "DoNotLock" true)
                (Default|SetupStoryDisplay (Variables|UI|GetUI_ReadStory) _title _author)
                (CallFunction|UpdateStoryDisplay)
                (Variables|UI|SetCurrentUI (Variables|UI|GetUI_ReadStory)))
              (:else)))
          (:then_1
            (bind _currentstory (Variables|Story|GetCurrentStory)
              (:then
                (if (Utilities|IsValid (Class|Story|VariablesState _currentstory))
                  (if (Utilities|Array|ContainsItem (Class|VariablesState|GetVariables (Class|Story|VariablesState _currentstory)) "trust")
                    (Class|Story|ObserveVariable (Variables|Story|GetCurrentStory) "trust" (EventDispatchers|CreateEvent :!event Custom|UpdateVariableTracking))
                    (CallFunction|UpdateTrust))))
              (:else))))
        (else
          (Development|PrintString (Utilities|String|Append "Error: Cannot find Tell Story camera for " (Utilities|String|ToString(Name) (Variables|Story|GetCurrentStoryRowname))) true true "(R=1.000000,G=0.000000,B=0.000000,A=1.000000)" 1e+01))))))

(event Custom|UpdateVariableTracking
  (params (variableName :type String) (newValue :type Ink%20Var%20Structure))
  (if (Utilities|Enum|Equal(Enum) variableName "trust")
    (CallFunction|UpdateTrust)))

(event Custom|ClearVariableTracking
  (bind _currentstory (Variables|Story|GetCurrentStory)
    (:then
      (if (Utilities|IsValid (Class|Story|VariablesState _currentstory))
        (if (Utilities|Array|ContainsItem (Class|VariablesState|GetVariables (Class|Story|VariablesState _currentstory)) "trust")
          (Class|Story|RemoveVariableObserver (Variables|Story|GetCurrentStory) (EventDispatchers|CreateEvent :!event Custom|UpdateVariableTracking) "trust"))))
    (:else)))

(event Custom|SelectChoice
  (params (ChoiceIndex :type Integer))
  (bind _currentstory (Variables|Story|GetCurrentStory)
    (:then
      (Class|Story|ChooseChoiceIndex _currentstory ChoiceIndex)
      (CallFunction|UpdateStoryDisplay))
    (:else)))

(event Custom|UpdateStoryDisplay
  (bind _currentstory (Variables|Story|GetCurrentStory)
    (:then
      (if (Class|Story|CanContinue _currentstory)
        (bind _returnvalue (Class|Story|ContinueMaximally (Variables|Story|GetCurrentStory)))
        (bind (_displaystring _commands) (CallFunction|ProcessIncomingString _returnvalue))
        (Utilities|FlowControl|Sequence
          (:then_0
            (bind _ui_readstory (Variables|UI|GetUI_ReadStory)
              (:then
                (Default|AddTexttoLog _ui_readstory (Utilities|Text|ToText(String) _displaystring))
                (bind _returnvalue_2 (Class|Story|CurrentChoices (Variables|Story|GetCurrentStory)))
                (if (> (Utilities|Array|Length _returnvalue_2) 0)
                  (for (_array_element _array_index) _returnvalue_2
                    (Default|AddChoice (Variables|UI|GetUI_ReadStory) (Utilities|Text|ToText(String) (Class|Choice|Text _array_element)) _array_index))
                  (else
                    (Default|AddEndOfStory (Variables|UI|GetUI_ReadStory)))))
              (:else)))
          (:then_1
            (if (> (Utilities|Array|Length _commands) 0)
              (CallFunction|CheckCommands _commands))))))
    (:else)))

(event Custom|ChangeMusicToMain
  (bind _musicmixalpha (Timeline|Timeline_ChangeMusic Reverse)
    (:Update
      (bind _mainmusicemitter (Variables|Default|GetMainMusicEmitter)
        (:then
          (Audio|Parameter|SetFloatParameter _mainmusicemitter "MusicMixAlpha" _musicmixalpha :!class /Script/Engine.AudioComponent))
        (:else)))))

(event Custom|ChangeMusicToStory
  (bind _musicmixalpha (Timeline|Timeline_ChangeMusic Play)
    (:Update
      (bind _mainmusicemitter (Variables|Default|GetMainMusicEmitter)
        (:then
          (Audio|Parameter|SetFloatParameter _mainmusicemitter "MusicMixAlpha" _musicmixalpha :!class /Script/Engine.AudioComponent))
        (:else)))))

(event Custom|ChangeCampfire
  (params (NewColor :type String))
  (Variables|Default|GetCampfireEmitter
    (:then
      (bind _returnvalue (Utilities|GetDataTableRow "/Game/Data/Data_CampfireColors.Data_CampfireColors" (Utilities|String|StringToName NewColor))
        (:then
          (Effects|Components|ParticleSystem|SetVectorParameter (Variables|Default|GetCampfireEmitter) "FlameColor" (Math|Conversions|ToVector(LinearColor) (.FlameColor (Utilities|Struct|BreakS_CampfireColors _returnvalue))))
          (Effects|Components|ParticleSystem|SetVectorParameter (Variables|Default|GetCampfireEmitter) "EmberColor" (* (Math|Conversions|ToVector(LinearColor) (.FlameColor (Utilities|Struct|BreakS_CampfireColors _returnvalue))) 5.0))
          (Effects|Components|ParticleSystem|SetVectorParameter (Variables|Default|GetCampfireEmitter) "SmokeColor" (Math|Conversions|ToVector(LinearColor) (.SmokeColor (Utilities|Struct|BreakS_CampfireColors _returnvalue))))
          (Effects|Components|ParticleSystem|SetVectorParameter (Variables|Default|GetCampfireEmitter) "LightColor" (Math|Conversions|ToVector(LinearColor) (.LightColor (Utilities|Struct|BreakS_CampfireColors _returnvalue)))))
        (:RowNotFound
          (Development|PrintString (Utilities|String|Append "Error: No color entry for \"" NewColor "\"") true true "(R=1.000000,G=0.000000,B=0.000000,A=1.000000)" 1e+01)
          (CallFunction|ResetCampfire))))
    (:else
      (Development|PrintString "Error: Campfire emitter is not valid" true true "(R=1.000000,G=0.000000,B=0.000000,A=1.000000)" 1e+01))))

(event Custom|ResetCampfire
  (CallFunction|ChangeCampfire "Default"))

(event Custom|ShowStoryImageLeft
  (params (ImageName :type String))
  (bind _returnvalue (Utilities|GetDataTableRow "/Game/Data/Data_StoryImages.Data_StoryImages" (Utilities|String|StringToName ImageName))
    (:then
      (bind _ui_readstory (Variables|UI|GetUI_ReadStory)
        (:then
          (Default|ShowImageLeft _ui_readstory (Utilities|Struct|BreakS_StoryImage _returnvalue)))
        (:else)))
    (:RowNotFound
      (Development|PrintString (Utilities|String|Append "Error: cannot fine image for \"" ImageName "\"") true true "(R=1.000000,G=0.000000,B=0.000000,A=1.000000)" 1e+01))))

(event Custom|ShowStoryImageRight
  (params (ImageName :type String))
  (bind _returnvalue (Utilities|GetDataTableRow "/Game/Data/Data_StoryImages.Data_StoryImages" (Utilities|String|StringToName ImageName))
    (:then
      (bind _ui_readstory (Variables|UI|GetUI_ReadStory)
        (:then
          (Default|ShowImageRight _ui_readstory (Utilities|Struct|BreakS_StoryImage _returnvalue)))
        (:else)))
    (:RowNotFound
      (Development|PrintString (Utilities|String|Append "Error: cannot fine image for \"" ImageName "\"") true true "(R=1.000000,G=0.000000,B=0.000000,A=1.000000)" 1e+01))))

(event Custom|HideImageLeft
  (bind _ui_readstory (Variables|UI|GetUI_ReadStory)
    (:then
      (Default|HideImageLeft _ui_readstory))
    (:else)))

(event Custom|HideImageRight
  (bind _ui_readstory (Variables|UI|GetUI_ReadStory)
    (:then
      (Default|HideImageRight _ui_readstory))
    (:else)))

(event Custom|PlayStorySound
  (params (SoundName :type String))
  (bind _returnvalue (Utilities|GetDataTableRow "/Game/Data/Data_StorySounds.Data_StorySounds" (Utilities|String|StringToName SoundName))
    (:then
      (bind _object (Utilities|AsyncLoadAsset (.SoundCue (Utilities|Struct|BreakS_StorySound _returnvalue)))
        (:Completed
          (bind _assound_cue (Utilities|Casting|CastToSoundCue _object))
          (Audio|PlaySound2D _assound_cue 1.0 1.0 0.0 0 0))))
    (:RowNotFound
      (Development|PrintString (Utilities|String|Append "Error: cannot fine sound for \"" SoundName "\"") true true "(R=1.000000,G=0.000000,B=0.000000,A=1.000000)" 1e+01))))

(event Custom|ShowTrust
  (bind _ui_readstory (Variables|UI|GetUI_ReadStory)
    (:then
      (bind _ui_trust (Variables|/Game/BP/UI/Story/UI_ReadStory.UI_ReadStory_C|GetUI_Trust _ui_readstory)
        (:then
          (Class|IUI|UI-Show(Message) _ui_trust))
        (:else)))
    (:else)))

(event Custom|HideTrust
  (bind _ui_readstory (Variables|UI|GetUI_ReadStory)
    (:then
      (bind _ui_trust (Variables|/Game/BP/UI/Story/UI_ReadStory.UI_ReadStory_C|GetUI_Trust _ui_readstory)
        (:then
          (Class|IUI|UI-Hide(Message) _ui_trust))
        (:else)))
    (:else)))

(event Custom|UpdateTrust
  (bind _currentstory (Variables|Story|GetCurrentStory)
    (:then
      (bind _ui_readstory (Variables|UI|GetUI_ReadStory)
        (:then
          (bind _ui_trust (Variables|/Game/BP/UI/Story/UI_ReadStory.UI_ReadStory_C|GetUI_Trust _ui_readstory)
            (:then
              (Default|UpdateTrust _ui_trust (Utilities|Struct|BreakInkVar (Class|VariablesState|GetVariable (Class|Story|VariablesState _currentstory) "trust"))))
            (:else)))
        (:else)))
    (:else)))

(fn ConstructionScript)

(fn CheckCommands
  (params (Commands :type Array%20of%20Strings))
  (for _array_element Commands
    (LocalVariables|SetCheckCommandString _array_element)
    (bind _array_element_2 (Utilities|Array|ForEachLoopwithBreak (Variables|Default|GetKnownCommands) :!label _label)
      (:LoopBody
        (if (Utilities|String|Contains (LocalVariables|GetCheckCommandString) _array_element_2)
          (LocalVariables|SetCommandToRun _array_element_2)
          (LocalVariables|SetIndexLeft (+ (Utilities|String|FindSubstring (LocalVariables|GetCheckCommandString) "(") 1))
          (LocalVariables|SetIndexRight (Utilities|String|FindSubstring (LocalVariables|GetCheckCommandString) ")"))
          (LocalVariables|SetCommandParameter (Utilities|String|GetSubstring (LocalVariables|GetCheckCommandString) (LocalVariables|GetIndexLeft) (- (LocalVariables|GetIndexRight) (LocalVariables|GetIndexLeft))))
          (goto _label Break)))
      (:Completed
        (CallFunction|RunCommand (LocalVariables|GetCommandToRun) (LocalVariables|GetCommandParameter)))))
  (return))

(fn RunCommand
  (params (Command :type String) (Parameter :type String))
  (switch string Command
    (:Default
      _)
    (:ShowImageLeft
      (CallFunction|ShowStoryImageLeft Parameter)
      (return))
    (:HideImageLeft
      (CallFunction|HideImageLeft)
      (return))
    (:ShowImageRight
      (CallFunction|ShowStoryImageRight Parameter)
      (return))
    (:HideImageRight
      (CallFunction|HideImageRight)
      (return))
    (:PlaySound
      (CallFunction|PlayStorySound Parameter)
      (return))
    (:ChangeMusic
      _)
    (:ChangeCampfire
      (CallFunction|ChangeCampfire Parameter)
      (return))
    (:ResetCampfire
      (CallFunction|ResetCampfire)
      (return))
    (:UseNarratorCamera
      _)
    (:UseSceneCamera
      _)
    (:show_trust
      (CallFunction|ShowTrust)
      (return))
    (:hide_trust
      (CallFunction|HideTrust)
      (return)))
  (return))

(fn ProcessIncomingString
  (params (InkString :type String))
  (LocalVariables|SetTestString InkString)
  (if (Utilities|String|Contains (LocalVariables|GetTestString) ">>>") :!label _label
    (LocalVariables|SetSearchIndex -1)
    (LocalVariables|SetSearchIndex (Utilities|String|FindSubstring (LocalVariables|GetTestString) ">>>" false false (LocalVariables|GetSearchIndex)))
    (LocalVariables|SetEndOfCommandIndex (Utilities|String|FindSubstring (LocalVariables|GetTestString) ")" false false (LocalVariables|GetSearchIndex)))
    (if (> (LocalVariables|GetEndOfCommandIndex) (LocalVariables|GetSearchIndex))
      (Math|Integer|IncrementInt (LocalVariables|GetEndOfCommandIndex)
        (:%20%20
          (bind _output_get (LocalVariables|SetCommandString (Utilities|String|GetSubstring (LocalVariables|GetTestString) (+ (LocalVariables|GetSearchIndex) 3) (- (LocalVariables|GetEndOfCommandIndex) (+ (LocalVariables|GetSearchIndex) 3)))))
          (Utilities|Array|Add (LocalVariables|GetCommandStrings) _output_get)
          (Utilities|Array|Add (LocalVariables|GetStringsToDisplay) (Utilities|String|TrimTrailing (Utilities|String|Trim (Utilities|String|GetSubstring (LocalVariables|GetTestString) 0 (- (LocalVariables|GetSearchIndex) 1)))))
          (LocalVariables|SetTestString (Utilities|String|RightChop (LocalVariables|GetTestString) (LocalVariables|GetEndOfCommandIndex)))
          (goto _label)))
      (else
        (Development|PrintString (Utilities|String|Append "Error: Command is incorrectly formatted in \"" (LocalVariables|GetTestString) "\"") true true "(R=1.000000,G=0.000000,B=0.000000,A=1.000000)" 1e+01)
        (return (LocalVariables|GetTestString) (LocalVariables|GetCommandStrings))))
    (else
      (Utilities|Array|Add (LocalVariables|GetStringsToDisplay) (LocalVariables|GetTestString))
      (return (Utilities|String|JoinStringArray (LocalVariables|GetStringsToDisplay) " ") (LocalVariables|GetCommandStrings)))))