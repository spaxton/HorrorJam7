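; Player controller for the Ink story game that handles startup, quitting and music switching.
; On BeginPlay it holds a black screen, turns on VSync, fades in, sends the game mode a start message and shows the mouse cursor.
; The Quit action and number keys plus M send messages to the game mode to quit or switch to named music tracks.
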(event EventBeginPlay
  (Class|PlayerCameraManager|SetManualCameraFade :self (Variables|Default|GetPlayerCameraManager) :InFadeAmount 1.0)
  (bind _returnvalue (Settings|GetGameUserSettings))
  (Class|GameUserSettings|SetVSyncEnabled _returnvalue true)
  (Class|GameUserSettings|ApplySettings _returnvalue true)
  (Utilities|FlowControl|Delay 0.1)
  (CameraFades|StartCameraFade :self (Variables|Default|GetPlayerCameraManager) :FromAlpha 1.0 :Duration 0.5)
  (Utilities|FlowControl|Delay 0.25)
  (Class|IStoryGameMode|GM-Start(Message) (Game|GetGameMode))
  (Variables|Default|SetbShowMouseCursor true))

(event Input|ActionEvents|InputActionQuit
  (params (Key :type Key%20Structure :default "None"))
  (:Pressed
    (Class|IStoryGameMode|GM-Quit(Message) (Game|GetGameMode))))

(event Input|KeyboardEvents|1
  (params (Key :type Key%20Structure :default "None"))
  (:Pressed
    (Class|IStoryGameMode|GM-SetMusic(Message) (Game|GetGameMode) "alpha_girl")))

(event Input|KeyboardEvents|2
  (params (Key :type Key%20Structure :default "None"))
  (:Pressed
    (Class|IStoryGameMode|GM-SetMusic(Message) (Game|GetGameMode) "alpha_terror")))

(event Input|KeyboardEvents|M
  (params (Key :type Key%20Structure :default "None"))
  (:Pressed
    (Class|IStoryGameMode|GM-SetMusic(Message) (Game|GetGameMode) "campfire")))

(event Input|KeyboardEvents|3
  (params (Key :type Key%20Structure :default "None"))
  (:Pressed
    (Class|IStoryGameMode|GM-SetMusic(Message) (Game|GetGameMode) "baddog_main1")))

(event Input|KeyboardEvents|4
  (params (Key :type Key%20Structure :default "None"))
  (:Pressed
    (Class|IStoryGameMode|GM-SetMusic(Message) (Game|GetGameMode) "baddog_alien")))

(event Input|KeyboardEvents|5
  (params (Key :type Key%20Structure :default "None"))
  (:Pressed
    (Class|IStoryGameMode|GM-SetMusic(Message) (Game|GetGameMode) "visitor_main")))

(event Input|KeyboardEvents|6
  (params (Key :type Key%20Structure :default "None"))
  (:Pressed
    (Class|IStoryGameMode|GM-SetMusic(Message) (Game|GetGameMode) "visitor_terror")))

(event Input|KeyboardEvents|7
  (params (Key :type Key%20Structure :default "None"))
  (:Pressed
    (Class|IStoryGameMode|GM-SetMusic(Message) (Game|GetGameMode) "hunger_main")))

(event Input|KeyboardEvents|0
  (params (Key :type Key%20Structure :default "None"))
  (:Pressed
    (Class|IStoryGameMode|GM-SetMusic(Message) (Game|GetGameMode) "tworings_terror")))

(event Input|KeyboardEvents|8
  (params (Key :type Key%20Structure :default "None"))
  (:Pressed
    (Class|IStoryGameMode|GM-SetMusic(Message) (Game|GetGameMode) "hunger_terror")))

(event Input|KeyboardEvents|9
  (params (Key :type Key%20Structure :default "None"))
  (:Pressed
    (Class|IStoryGameMode|GM-SetMusic(Message) (Game|GetGameMode) "tworings_main")))

(fn ConstructionScript)