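; BP_Narrator_LowPerf is a narrator actor Blueprint, named as a low-performance variant, that shows and hides a static mesh.
; The construction script runs the parent's, then applies the StaticMesh variable to the NarratorStaticMesh component.
; Fadein and FadeOut events toggle that component's visibility instantly, propagating to children, with no gradual fade.
; BeginPlay, overlap and Tick hold no active logic.
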(event EventBeginPlay
  (|CallParentFunction) ; This node is disabled and will not be called.\nDrag off pins to build functionality.
)

(event Collision|EventActorBeginOverlap
  (params (OtherActor :type Actor%20Object%20Reference)))

(event EventTick
  (params (DeltaSeconds :type Float%20%28single-precision%29)))

(event EventFadeOut
  (Rendering|SetVisibility (Variables|Default|GetNarratorStaticMesh) false true))

(event EventFadein
  (Rendering|SetVisibility (Variables|Default|GetNarratorStaticMesh) true true))

(fn ConstructionScript
  (|CallParentFunction)
  (Components|StaticMesh|SetStaticMesh (Variables|Default|GetNarratorStaticMesh) (Variables|Default|GetStaticMesh)))